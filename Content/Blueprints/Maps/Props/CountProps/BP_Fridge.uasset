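; BP_Fridge is a fridge prop with a cable tethered to another actor.
; Each tick it measures the distance from the mesh to the cable's attached actor through GetCustomLength.
; Once that distance passes a fixed threshold, it releases the cable's end attachment and hides the cable, as if unplugged.
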(event `self.ReceiveTick`
  (params (DeltaSeconds :type "Float (single-precision)"))
  (bind _cable (`self.Cable`))
  (if (> (`self.GetCustomLength`) 350.0)
    (set `CableComponent.bAttachEnd` false _cable)
    (`SceneComponent.SetVisibility` _cable false false)))

(fn `GetCustomLength`
  (returns (CurrentLength :type "Float (double-precision)"))
  (return (`KismetMathLibrary.VSize` (- (`self.K2_GetActorLocation` (`CableComponent.GetAttachedActor` (`self.Cable`))) (`SceneComponent.K2_GetComponentLocation` (`self.Mesh`))))))

(fn `UserConstructionScript`)